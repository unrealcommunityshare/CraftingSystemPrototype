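; Player controller that exposes debug keys for testing the inventory and crafting system.
; Pressing C asks InventoryComponent to craft a single IronArrow.
; Pressing I iterates the keys of the component's InventoryData map and prints each item name with its amount on screen.
; BeginPlay, Tick and the construction script are empty.
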(event EventBeginPlay)

(event EventTick
  (params (DeltaSeconds :type Float%20%28single-precision%29)))

(event Input|KeyboardEvents|C
  (params (Key :type Key%20Structure :default "None"))
  (:Pressed
    (Default|CraftSingleItem (Variables|Default|GetInventoryComponent) "IronArrow")))

(event Input|KeyboardEvents|I
  (params (Key :type Key%20Structure :default "None"))
  (bind _inventorycomponent (Variables|Default|GetInventoryComponent))
  (bind _inventorydata (Variables|/Game/Inventory/InventoryComponent.InventoryComponent_C|GetInventoryData _inventorycomponent))
  (:Pressed
    (bind _keys (Utilities|Map|Keys _inventorydata))
    (for _array_element _keys
      (Development|PrintString (Utilities|String|Append _array_element " = " (Utilities|String|ToString(Integer) (.amount (.Value (Utilities|Map|Find _inventorydata _array_element))))) true true "(R=0.000000,G=0.660000,B=1.000000,A=1.000000)" 5.0))))

(fn ConstructionScript)